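; AIChar_BP is an AI-controlled shooter character that takes damage and respawns at a random SpawnPoint actor.
; Damage lowers Health, and at zero the character teleports far below the world, then after a short delay resets health and moves to one of the spawn points gathered at BeginPlay.
; StartShooting runs a looping timer that spawns AIProj projectiles from an arrow component until StopShooting clears it, and HealthBonus sets health to a given maximum.
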(event Custom|AIShoot
  ;[0.15 0.15 0.15 0.5] AIShoot
  (Game|SpawnActorfromClass "/Game/AI/AIProj.AIProj_C" (Transformation|GetWorldTransform (Variables|Default|GetArrow1)) "Undefined" "MultiplyWithRoot" self 0))

(event Custom|StartShooting
  ;[0.15 0.15 0.15 0.5] Projectile
  (Utilities|Time|SetTimerbyFunctionName 0 "AIShoot" (Variables|Default|GetRateofFire) true))

(event Custom|StopShooting
  ;[0.15 0.15 0.15 0.5] Projectile
  (Utilities|Time|ClearTimerbyFunctionName 0 "AIShoot"))

(event Custom|CheckHealth
  ;[0.15 0.15 0.15 0.5] Health and Damage
  (if (<= (Variables|Default|GetHealth) 0.0)
    (Transformation|SetActorLocation "0.000000,0.000000,-5000.000000" false true)
    (CallFunction|Respawn)))

(event Custom|HealthBonus
  (params (Max%20Health :type Float%20%28double-precision%29))
  ;[0.15 0.15 0.15 0.5] Health and Damage
  (bind _output_get (Variables|Default|SetMax%20Health Max%20Health))
  (Variables|Default|SetHealth _output_get))

(event Custom|Respawn
  (bind _spawnpoints (Variables|Default|GetSpawnPoints))
  (Utilities|FlowControl|Delay 2.0)
  (Variables|Default|SetHealth 1e+02)
  (Transformation|SetActorLocation (Transformation|GetActorLocation (Utilities|Array|Get(acopy) _spawnpoints (Math|Random|RandomIntegerinRange 0 (- (Utilities|Array|Length _spawnpoints) 1)))) false true))

(event Game|Damage|EventAnyDamage
  (params (Damage :type Float%20%28single-precision%29) (DamageType :type Damage%20Type%20Object%20Reference) (InstigatedBy :type Controller%20Object%20Reference) (DamageCauser :type Actor%20Object%20Reference))
  ;[0.15 0.15 0.15 0.5] Health and Damage
  (Variables|Default|SetDamage%20Causer DamageCauser)
  (Variables|Default|SetHealth (- (Variables|Default|GetHealth) Damage))
  (CallFunction|CheckHealth)
  (Development|PrintString (Utilities|String|ToString(Float) (Variables|Default|GetHealth)) true true "(R=0.453125,G=0.068154,B=0.124847,A=1.000000)"))

(event EventBeginPlay
  (bind _outactors (Actor|GetAllActorsOfClass "/Game/Spawner/SpawnPoint.SpawnPoint_C"))
  (Variables|Default|SetSpawnPoints _outactors))

(fn ConstructionScript)